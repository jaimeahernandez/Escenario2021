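; Explosion ejection object that, when activated, launches a projectile component upward and detonates it at the end of its travel.
; BeginPlay caches the projectile's world position as the exit hole.
; Activate reveals the projectile and plays a timeline whose height curve, scaled by a maximum height, drives its relative Z.
; When the timeline finishes, it spawns explosion particles at the projectile and smoke at the origin, then destroys the component.
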(event `self.ReceiveBeginPlay`
  ;[1 1 1] Captura Posición Original del Proyectil (Orificio de Salida)
  (set `self.OriginProjectile` (`SceneComponent.K2_GetComponentLocation` (`self.Explosion_Projectile`))))

(event `self.Activate`
  (`SceneComponent.SetVisibility` (`self.Explosion_Projectile`) true false)
  (bind (_direction _altura) (`Timeline|Projectile_EjectionTLine` :!via `PlayFromStart`)
    (:`Update`
      (`SceneComponent.K2_SetRelativeLocation` (`self.Explosion_Projectile`) (`KismetMathLibrary.MakeVector` 0.0 0.0 (* _altura (`self.AlturaMAXProjectile`))) false false))
    (:`Finished`
      (`GameplayStatics.SpawnEmitterAtLocation` "/Game/MobileStarterContent/Particles/P_Explosion.P_Explosion" (`SceneComponent.K2_GetComponentLocation` (`self.Explosion_Projectile`)))
      (`GameplayStatics.SpawnEmitterAtLocation` "/Game/MobileStarterContent/Particles/P_Smoke.P_Smoke" (`self.OriginProjectile`))
      (`ActorComponent.K2_DestroyComponent` (`self.Explosion_Projectile`)))))

(fn `UserConstructionScript`
  (`parent.UserConstructionScript`))